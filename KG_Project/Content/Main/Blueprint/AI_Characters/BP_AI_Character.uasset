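; AI character Blueprint that walks a linked chain of waypoints after play begins.
; On BeginPlay it sets its desired gait from a preferred gait, then uses AIMoveTo toward the assigned GoToPoint.
; Each point references its NextPoint, so movement continues until the chain runs out.
; A failed move advances to the next point just like a successful one, rather than retrying.
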(event `self.ReceiveBeginPlay`
  (bind _go_to_point (`self.Go To Point`))
  (bind _next_point (`/Game/Main/Blueprint/Utils/BP_PatrolPoint.Next Point` (`self.Go To Point`)))
  (`parent.ReceiveBeginPlay`)
  (set `self.DesiredGait` (`self.Prefered Gait`))
  (`/Engine/EditorBlueprintResources/StandardMacros.IsValid` _go_to_point
    (:`Is Valid`
      (`|AIMoveTo` self (`self.K2_GetActorLocation` _go_to_point) null 5.0 true :!label _label
        (:`OnSuccess`
          _)
        (:`OnFail`
          _))
      (`/Engine/EditorBlueprintResources/StandardMacros.IsValid` _next_point
        (:`Is Valid`
          (set `self.Go To Point` _next_point)
          (goto _label))))))

(fn `UserConstructionScript`
  (`parent.UserConstructionScript`))