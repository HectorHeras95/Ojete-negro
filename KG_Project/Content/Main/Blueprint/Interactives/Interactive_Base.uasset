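; Base Blueprint for interactive objects that swaps an attached marker for the interactive's own billboard display.
; Activation reveals RootBillboard and its children, then hides and caches the first attached actor, provided it is a Marker_Base, and calls ChangeStyleInteractive.
; Deactivation hides the billboard hierarchy and restores the cached marker if valid.
; ChangeStyleInteractive, the construction script and the event graph are empty here.
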(event `self.ReceiveActorBeginOverlap`
  (params (OtherActor :type "Actor Object Reference")))

(fn `Activate Interactive`
  (`SceneComponent.SetHiddenInGame` (`self.RootBillboard`) false true)
  (for _array_element (`self.GetAttachedActors` false)
    (bind _asmarker_base (cast `/Game/Main/Blueprint/Markers/Marker_Base` _array_element))
    (bind _output_get (set `self.Current Marker Activate` _asmarker_base))
    (`/Game/Main/Blueprint/Markers/Marker_Base.Hide Marker` _output_get)
    (`self.Change Style Interactive`)
    (break)))

(fn `Change Style Interactive`)

(fn `Deactivate Interactive`
  (bind _current_marker_activate (`self.Current Marker Activate`))
  (`SceneComponent.SetHiddenInGame` (`self.RootBillboard`) true true)
  (`/Engine/EditorBlueprintResources/StandardMacros.IsValid` _current_marker_activate
    (:`Is Valid`
      (`/Game/Main/Blueprint/Markers/Marker_Base.Show Marker` _current_marker_activate))))

(fn `UserConstructionScript`)