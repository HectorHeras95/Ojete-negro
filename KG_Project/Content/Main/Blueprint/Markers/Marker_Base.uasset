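; Base actor for in-game markers, displayed through a Marker widget component.
; InitMarkerBP casts that component's widget to MarkerWidget and initializes it with the actor's TypeMarker.
; Helper functions show or hide the widget component or destroy the whole actor.
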(event `Init Marker BP`
  (bind _asmarker_widget (cast `/Game/Main/Blueprint/Markers/MarkerWidget` (`WidgetComponent.GetWidget` (`self.Marker`))))
  (`/Game/Main/Blueprint/Markers/MarkerWidget.InitMarker` _asmarker_widget (`self.TypeMarker`)))

(fn `Destroy Marker`
  (`self.K2_DestroyActor`))

(fn `Hide Marker`
  (`SceneComponent.SetHiddenInGame` (`self.Marker`) true false))

(fn `Show Marker`
  (`SceneComponent.SetHiddenInGame` (`self.Marker`) false false))

(fn `UserConstructionScript`)