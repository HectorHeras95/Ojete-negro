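; Mission_Base is a skeleton base Blueprint for missions that tracks a current step and supports saving and loading it.
; Save and load events copy CurrentStep to and from a VariablesToSave structure, printing the value for debugging.
; InitMission and the task and objective creation functions are empty stubs.
; BeginPlay only delays, while the LoadVariables call and the GameInstance and player character caching are disconnected.
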(event `self.ReceiveBeginPlay`
  (`KismetSystemLibrary.Delay` 1.0))

(event `Load_Variables`
  ;[1 0.1719 0.1719] Save System
  (bind _output_get (set `self.Current Step` (`.CurrentStep_36_3944AAA1458C0612FCD8E6A909CB226D` (break `/Game/Main/Blueprint/Missions/VariablesMIssion_Base` (`self.Variables To Save`)))))
  (`KismetSystemLibrary.PrintString` (`KismetStringLibrary.Conv_IntToString` _output_get)))

(event `Save Variables Inside Structure`
  ;[1 0.1719 0.1719] Save System
  (bind _output_get (set `self.Variables To Save` (make `/Game/Main/Blueprint/Missions/VariablesMIssion_Base` (`self.Current Step`))))
  (`KismetSystemLibrary.PrintString` (`KismetStringLibrary.Concat_StrStr` (`KismetStringLibrary.Conv_IntToString` (`.CurrentStep_36_3944AAA1458C0612FCD8E6A909CB226D` (break `/Game/Main/Blueprint/Missions/VariablesMIssion_Base` _output_get))) "       " "structura  Save Variables Inside Structure") true true (struct :`G` 0.66 :`B` 1.0 :`A` 1.0) 3.0))

(event `Init Mission`)

(fn `Create New Objective`
  (params (NewParam :type Text)))

(fn `Create New Task`)

(fn `UserConstructionScript`)