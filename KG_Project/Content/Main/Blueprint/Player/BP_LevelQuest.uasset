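; BP_LevelQuest is a level quest that tracks an ordered list of objectives and flags itself completed once the sequence finishes.
; On BeginPlay it binds NextObjective to the first objective's MarkedAsCompleted event and advances the index.
; Each completion binds the following objective the same way, or sets Completed when none remain.
; An empty list binds nothing, so Completed is never set in that case.
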(event `self.ReceiveBeginPlay`
  (bind _objectives (`self.Objectives`))
  (if (> (`KismetArrayLibrary.Array_Length` _objectives) 0)
    (add `/Game/Main/Blueprint/Player/BP_Objective.Marked As Completed` (`|GetArrayItem` _objectives (`self.Index Objective`)) (delegate `Next Objective`) :!label _label)
    (`/Engine/EditorBlueprintResources/StandardMacros.IncrementInt` (`self.Index Objective`))))

(event `Next Objective`
  (if (> (`KismetArrayLibrary.Array_Length` (`self.Objectives`)) (`self.Index Objective`))
    (goto _label)
    (else
      (set `self.Completed` true))))

(fn `UserConstructionScript`)