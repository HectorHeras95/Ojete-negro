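; BP_DynamicMesh is a Geometry Script generated-mesh actor, in a player testing folder, that builds a displaced mesh from a static mesh.
; On rebuild it copies the StaticMesh, applies PN tessellation and displaces it by a texture map.
; It then smooths the result, recomputes normals and plane-cuts it, with flipped side, just above negative half the displacement magnitude on Z.
; Displacement and all later steps require a valid DisplaceMap.
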(event `self.OnRebuildGeneratedMesh`
  (params (TargetMesh :type "DynamicMesh Object Reference"))
  (bind _static_mesh (`self.Static Mesh`)
    (:`then`
      (bind _returnvalue (`GeometryScriptLibrary_StaticMeshFunctions.CopyMeshFromStaticMesh` _static_mesh TargetMesh (struct) (struct) null)
        (:`Success`
          (bind _returnvalue_2 (`GeometryScriptLibrary_MeshSubdivideFunctions.ApplyPNTessellation` _returnvalue (struct) (`self.Tessellation Level`) null))
          (bind _displace_map (`self.Displace Map`)
            (:`then`
              (bind _returnvalue_3 (`GeometryScriptLibrary_MeshDeformFunctions.ApplyDisplaceFromTextureMap` _returnvalue_2 _displace_map (make `GeometryScriptDisplaceFromTextureOptions` (`self.Displace Magnitude`)) 0 null))
              (bind _returnvalue_4 (`GeometryScriptLibrary_MeshDeformFunctions.ApplyIterativeSmoothingToMesh` _returnvalue_3 (make `GeometryScriptIterativeMeshSmoothingOptions` 6 2.0) null))
              (bind _returnvalue_5 (`GeometryScriptLibrary_MeshNormalsFunctions.RecomputeNormals` _returnvalue_4 (struct) null))
              (`GeometryScriptLibrary_MeshBooleanFunctions.ApplyMeshPlaneCut` _returnvalue_5 (`KismetMathLibrary.MakeTransform` (`KismetMathLibrary.MakeVector` 0.0 0.0 (+ (* (/ (`self.Displace Magnitude`) 2.0) -1.0) 0.1))) (make `GeometryScriptMeshPlaneCutOptions` true true true) null))
            (:`else`)))))
    (:`else`)))

(fn `UserConstructionScript`)