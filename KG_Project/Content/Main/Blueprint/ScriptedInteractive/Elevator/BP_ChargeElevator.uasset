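; Charge elevator, a child of a parent elevator Blueprint, that adds a ramp which closes on a timer.
; BeginPlay runs MovementFinish, which only calls the parent version.
; ActivateRamp binds player overlap events and starts the close timer on opening, setting Ramp visibility from OpenDoorTrue rather than OpenRampTrue.
; Closing waits while the player is on the ramp, retrying when they step off after the timer expires.
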(event `self.ReceiveBeginPlay`
  (`self.MovementFinish`))

(event `self.MovementFinish`
  (`parent.MovementFinish`))

(event `Activate Ramp`
  (params (Open :type Boolean))
  (bind _output_get (set `self.OpenRampTrue` Open))
  (if _output_get
    (`SceneComponent.SetVisibility` (`self.Ramp`) (`self.OpenDoorTrue`) true :!label _label)
    (if (`self.OpenRampTrue`)
      (add `PrimitiveComponent.OnComponentBeginOverlap` (`self.CollisionRamp`) (`|CreateDelegate` :!event `BeginTriggerRamp`))
      (add `PrimitiveComponent.OnComponentEndOverlap` (`self.CollisionRamp`) (`|CreateDelegate` :!event `EndTriggerRamp`))
      (bind _returnvalue (`KismetSystemLibrary.K2_SetTimerDelegate` (delegate `TimerCloseRamp`) (`self.TimeToCloseRamp`)))
      (set `self.HandleTimerCloseRamp` _returnvalue))
    (elif (not (`self.IsOnTheRamp`))
      (remove `PrimitiveComponent.OnComponentBeginOverlap` (`self.CollisionRamp`) (`|CreateDelegate` :!event `BeginTriggerRamp`))
      (remove `PrimitiveComponent.OnComponentEndOverlap` (`self.CollisionRamp`) (`|CreateDelegate` :!event `EndTriggerRamp`))
      (goto _label))))

(event `TimerCloseRamp`
  (`self.Activate Ramp` false))

(event `BeginTriggerRamp`
  (params (OverlappedComponent :type "PrimitiveComponent Object Reference") (OtherActor :type "Actor Object Reference") (OtherComp :type "PrimitiveComponent Object Reference") (OtherBodyIndex :type Integer) (bFromSweep :type Boolean) (SweepResult :type "HitResult Structure (by ref)"))
  (cast `/Game/Main/Blueprint/Player/BP_PlayerCharacter_KG` OtherActor)
  (set `self.IsOnTheRamp` true))

(event `EndTriggerRamp`
  (params (OverlappedComponent :type "PrimitiveComponent Object Reference") (OtherActor :type "Actor Object Reference") (OtherComp :type "PrimitiveComponent Object Reference") (OtherBodyIndex :type Integer))
  (cast `/Game/Main/Blueprint/Player/BP_PlayerCharacter_KG` OtherActor)
  (set `self.IsOnTheRamp` false)
  (if (not (`KismetSystemLibrary.K2_IsTimerActiveHandle` (`self.HandleTimerCloseRamp`)))
    (`self.Activate Ramp` false)))

(fn `UserConstructionScript`
  (`parent.UserConstructionScript`))