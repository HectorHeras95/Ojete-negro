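; Base elevator actor that moves its Elevator component between the PointA and PointB markers.
; ActivateElevator scales the MovementElevator timeline's play rate so the trip lasts TimeToMove, then plays it from the start.
; Each update sweeps the component along a world-space lerp, from A to B when GoUp is true and reversed otherwise.
; On completion it calls MovementFinish, which is an empty event here.
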(event `Activate Elevator`
  (params (GoUp :type Boolean))
  (bind _movement_elevator (`self.Movement Elevator`))
  (bind _returnvalue (`SceneComponent.K2_GetComponentLocation` (`self.PointB`)))
  (bind _returnvalue_2 (`SceneComponent.K2_GetComponentLocation` (`self.PointA`)))
  (`TimelineComponent.SetPlayRate` _movement_elevator (/ (`TimelineComponent.GetTimelineLength` _movement_elevator) (`self.TimeToMove`)))
  (bind (_direction _alpha_location) (`Timeline|Movement Elevator` :`NewTime` 0.0 :!via `PlayFromStart`)
    (:`Update`
      (`SceneComponent.K2_SetWorldLocation` (`self.Elevator`) (`KismetMathLibrary.SelectVector` (`KismetMathLibrary.VLerp` _returnvalue_2 _returnvalue _alpha_location) (`KismetMathLibrary.VLerp` _returnvalue _returnvalue_2 _alpha_location) GoUp) true false))
    (:`Finished`
      (`self.MovementFinish`))))

(event `MovementFinish`)

(fn `UserConstructionScript`)