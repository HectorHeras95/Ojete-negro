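; Glass-building elevator, a child Blueprint that adds a ramp and two swinging doors when the elevator finishes moving.
; On arrival, timelines scale the ramp out and rotate the doors open.
; Once extended, the ramp binds overlap events and starts a close timer.
; Closing waits while the player is on the ramp; leaving after the timer expires retracts it and shuts the doors.
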(event `self.MovementFinish`
  (`parent.MovementFinish`)
  (`self.Activate Ramp` true)
  (`self.Activate Doors` true))

(event `Activate Doors`
  (params (Open :type Boolean))
  (if Open
    (bind (_direction _door_a _door_b) (`Timeline|OpenDoors` :!label _label)
      (:`Update`
        (`SceneComponent.K2_SetRelativeRotation` (`self.Door A`) (`KismetMathLibrary.MakeRotator` 0.0 0.0 _door_a) false false)
        (`SceneComponent.K2_SetRelativeRotation` (`self.Door B`) (`KismetMathLibrary.MakeRotator` 0.0 0.0 _door_b) false false)))
    (else
      (goto _label :!via `Reverse`))))

(event `Activate Ramp`
  (params (Open :type Boolean))
  (bind _ramp (`self.Ramp`))
  (bind (_relativescale3d_x _relativescale3d_y _relativescale3d_z) (`KismetMathLibrary.BreakVector` (`SceneComponent.RelativeScale3D` _ramp)))
  (bind _output_get (set `self.OpenRampTrue` Open))
  (if _output_get
    (bind (_direction _scaleramp) (`Timeline|OpenRamp` :!label _label_2)
      (:`Update`
        (`SceneComponent.SetRelativeScale3D` _ramp (`KismetMathLibrary.MakeVector` _scaleramp _relativescale3d_y _relativescale3d_z)))
      (:`Finished`
        (if (`self.OpenRampTrue`)
          (`self.Activate Doors` true)
          (add `PrimitiveComponent.OnComponentBeginOverlap` (`self.CollisionRamp`) (`|CreateDelegate` :!event `BeginTriggerRamp`))
          (add `PrimitiveComponent.OnComponentEndOverlap` (`self.CollisionRamp`) (`|CreateDelegate` :!event `EndTriggerRamp`))
          (bind _returnvalue (`KismetSystemLibrary.K2_SetTimerDelegate` (delegate `TimerCloseRamp`) (`self.TimeToCloseRamp`)))
          (set `self.HandleTimerCloseRamp` _returnvalue))))
    (elif (not (`self.IsOnTheRamp`))
      (remove `PrimitiveComponent.OnComponentBeginOverlap` (`self.CollisionRamp`) (`|CreateDelegate` :!event `BeginTriggerRamp`))
      (remove `PrimitiveComponent.OnComponentEndOverlap` (`self.CollisionRamp`) (`|CreateDelegate` :!event `EndTriggerRamp`))
      (goto _label_2 :!via `Reverse`))))

(event `TimerCloseRamp`
  (`self.Activate Ramp` false)
  (if (not (`self.IsOnTheRamp`))
    (`self.Activate Doors` false)))

(event `BeginTriggerRamp`
  (params (OverlappedComponent :type "PrimitiveComponent Object Reference") (OtherActor :type "Actor Object Reference") (OtherComp :type "PrimitiveComponent Object Reference") (OtherBodyIndex :type Integer) (bFromSweep :type Boolean) (SweepResult :type "HitResult Structure (by ref)"))
  (cast `/Game/Main/Blueprint/Player/BP_PlayerCharacter_KG` OtherActor)
  (set `self.IsOnTheRamp` true))

(event `EndTriggerRamp`
  (params (OverlappedComponent :type "PrimitiveComponent Object Reference") (OtherActor :type "Actor Object Reference") (OtherComp :type "PrimitiveComponent Object Reference") (OtherBodyIndex :type Integer))
  (cast `/Game/Main/Blueprint/Player/BP_PlayerCharacter_KG` OtherActor)
  (set `self.IsOnTheRamp` false)
  (if (not (`KismetSystemLibrary.K2_IsTimerActiveHandle` (`self.HandleTimerCloseRamp`)))
    (`self.Activate Ramp` false)
    (`self.Activate Doors` false)))

(fn `UserConstructionScript`
  (`parent.UserConstructionScript`))