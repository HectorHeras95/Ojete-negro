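; BP_SplineSpawner is an actor that spawns an actor and moves it along its spline.
; On activation, optionally at BeginPlay, it waits a random delay, then spawns the actor if none is set.
; A timeline with randomized duration, swappable float curves and optional looping drives swept movement, sampling location and rotation at separate distances along the spline.
; An empty FinishSpline event fires when the timeline finishes.
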(event `self.ReceiveBeginPlay`
  (if (`self.AutoActivate`)
    (`self.ActivateMovement`)))

(event `ActivateMovement`
  (bind _movementactortospline (`self.MovementActorToSpline`))
  (bind _spline (`self.Spline`))
  (bind _returnvalue (`SplineComponent.GetSplineLength` _spline))
  (`KismetSystemLibrary.Delay` (`KismetMathLibrary.RandomFloatInRange` (`self.Min Delay after activate`) (`self.Max Delay after activate`)))
  (`self.ActorToMove`
    (:`then`
      _)
    (:`else`
      (bind _returnvalue_2 (`|SpawnActorFromClass` (`self.ActorToSpawn`) (`SplineComponent.GetTransformAtSplinePoint` (`self.Spline`) 0 "Local" false) "Undefined" "OverrideRootScale" null null))
      (set `self.ActorToMove` _returnvalue_2)))
  (`TimelineComponent.SetPlayRate` _movementactortospline (/ 1.0 (`KismetMathLibrary.RandomFloatInRange` (`self.Min Duration`) (`self.Max Duration`))))
  (`TimelineComponent.SetFloatCurve` _movementactortospline (`self.Float Curve Location`) "Location")
  (`TimelineComponent.SetFloatCurve` _movementactortospline (`self.Float Curve Rotation`) "Rotation")
  (`TimelineComponent.SetLooping` (`self.MovementActorToSpline`) (`self.Is Loop`))
  (bind (_direction _location _rotation) (`Timeline|MovementActorToSpline` :!via `PlayFromStart`)
    (:`Update`
      (set `self.Alpha_L1` _location)
      (set `self.Alpha_R1` _rotation)
      (`self.K2_SetActorLocationAndRotation` (`self.ActorToMove`) (`SplineComponent.GetLocationAtDistanceAlongSpline` _spline (`KismetMathLibrary.Lerp` 0.0 _returnvalue (`self.Alpha_L1`)) "World") (`SplineComponent.GetRotationAtDistanceAlongSpline` _spline (`KismetMathLibrary.Lerp` 0.0 _returnvalue (`self.Alpha_R1`)) "World") true false))
    (:`Finished`
      (`self.FinishSpline`))))

(event `FinishSpline`)

(fn `UserConstructionScript`)