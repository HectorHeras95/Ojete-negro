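; BP_Spline_Mesh is a construction-script spline actor that lays a static mesh along a spline path.
; It adds one collidable spline mesh component per segment between points, applying shared forward axis, roll, scale and mesh settings.
; The segment count comes from Spline, while local positions and tangents come from SplineTrack.
; The parent construction script runs inside the loop, once per segment, and the event graph is unused.
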(fn `UserConstructionScript`
  (bind _splinetrack (`self.SplineTrack`))
  (bind _scale (`self.Scale`))
  (bind _returnvalue (`KismetMathLibrary.DegreesToRadians` (`self.Roll`)))
  (for _index (range (+ (- (`SplineComponent.GetNumberOfSplinePoints` (`self.Spline`)) 2) 1))
    (bind _returnvalue_2 (`AddComponent|NODE_AddSplineMeshComponent-0`))
    (`SplineMeshComponent.SetForwardAxis` _returnvalue_2 (`self.ForwardAxis`) true)
    (`SplineMeshComponent.SetEndRoll` _returnvalue_2 _returnvalue true)
    (`SplineMeshComponent.SetStartRoll` _returnvalue_2 _returnvalue true)
    (`SplineMeshComponent.SetStartScale` _returnvalue_2 _scale true)
    (`SplineMeshComponent.SetEndScale` _returnvalue_2 _scale true)
    (`StaticMeshComponent.SetStaticMesh` _returnvalue_2 (`self.StaticMesh`))
    (`PrimitiveComponent.SetCollisionEnabled` _returnvalue_2 "QueryAndPhysics")
    (bind _returnvalue_3 (+ _index 1))
    (`SplineMeshComponent.SetStartAndEnd` _returnvalue_2 (`SplineComponent.GetLocationAtSplinePoint` _splinetrack _index "Local") (`SplineComponent.GetTangentAtSplinePoint` _splinetrack _index "Local") (`SplineComponent.GetLocationAtSplinePoint` _splinetrack _returnvalue_3 "Local") (`SplineComponent.GetTangentAtSplinePoint` _splinetrack _returnvalue_3 "Local") true)
    (`parent.UserConstructionScript`)))