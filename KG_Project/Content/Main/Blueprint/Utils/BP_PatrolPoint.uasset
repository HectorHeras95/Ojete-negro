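; BP_PatrolPoint is a patrol route marker that visually links to the next point in the route through its NextPoint reference.
; When NextPoint is valid, the construction script rotates the Connection component toward it and scales its X axis by the distance to span the gap.
; The event graph has no active logic, and its hide-in-game call is never executed.
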(event `self.ReceiveBeginPlay`)

(fn `UserConstructionScript`
  (bind _next_point (`self.Next Point`))
  (bind _connection (`self.Connection`))
  (bind _returnvalue (`SceneComponent.K2_GetComponentLocation` _connection))
  (bind _returnvalue_2 (`self.K2_GetActorLocation` _next_point))
  (bind (_returnvalue_x _returnvalue_y _returnvalue_z) (`KismetMathLibrary.BreakVector` (`SceneComponent.K2_GetComponentScale` (`self.Connection`))))
  (`/Engine/EditorBlueprintResources/StandardMacros.IsValid` _next_point
    (:`Is Valid`
      (`SceneComponent.K2_SetWorldRotation` _connection (`KismetMathLibrary.FindLookAtRotation` _returnvalue _returnvalue_2) false false)
      (`SceneComponent.SetWorldScale3D` _connection (`KismetMathLibrary.MakeVector` (/ (`KismetMathLibrary.Vector_Distance` _returnvalue _returnvalue_2) 80.0) _returnvalue_y _returnvalue_z)))))