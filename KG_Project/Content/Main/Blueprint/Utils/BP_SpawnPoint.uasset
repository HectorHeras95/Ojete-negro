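; Spawn point actor that creates a BP_AI_Character at its own transform, on BeginPlay if AutoStart is set or whenever SpawnUnit is called.
; Each spawned character receives a GoToPoint from PatrolPoints, picked at random or in wrapping sequence depending on RandomizePatrols.
; It binds to each character's death event and re-broadcasts it through its own AICharacterDeath dispatcher.
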(event `self.ReceiveBeginPlay`
  (if (`self.Auto Start`)
    (`self.Spawn Unit`)))

(event `Spawn Unit`
  (bind _returnvalue (`|SpawnActorFromClass` "/Game/Main/Blueprint/AI_Characters/BP_AI_Character.BP_AI_Character_C" (`self.GetTransform`) "Undefined" "OverrideRootScale" null (`self.Get Next Patrol`) null))
  (add `/Game/Main/Blueprint/AI_Characters/BP_AI_Character.AI Character Death` _returnvalue (delegate `Dispatch Spawn Death`)))

(event `Dispatch Spawn Death`
  (`self.AI Character Death`))

(fn `Get Next Patrol`
  (returns (`Patrol Point` :type "/Game/Main/Blueprint/Utils/BP_PatrolPoint Object Reference"))
  (locals (`Result Patrol` :type "/Game/Main/Blueprint/Utils/BP_PatrolPoint Object Reference"))
  (bind _patrol_points (`self.Patrol Points`))
  (bind _current_patrol (`self.Current Patrol`))
  (if (`self.Randomize Patrols`)
    (set `local.Result Patrol` (`KismetArrayLibrary.Array_Random` (`self.Patrol Points`)))
    (else
      (set `local.Result Patrol` (`|GetArrayItem` _patrol_points (`self.Current Patrol`)))
      (`/Engine/EditorBlueprintResources/StandardMacros.IncrementInt` _current_patrol
        (:`  `
          (if (> _current_patrol (`KismetArrayLibrary.Array_LastIndex` _patrol_points))
            (set `self.Current Patrol` 0))))))
  (return (`local.Result Patrol`)))

(fn `UserConstructionScript`)