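; Wave manager that spawns AI enemy waves after an alarm, capped by a maximum alive count.
; Randomized timers schedule waves, whose random size can grow by increments, with pause, resume, reset and retiming controls.
; The spawn loop picks random group points and tracks deaths to update the alive count.
; As written, InitWaves clears SpawnGroups without refilling it, so it only reschedules and never reaches that loop.
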(event `self.ReceiveBeginPlay`
  (if (not true)
    (set `self.Init Min Enemies Per Wave` (`self.Min Spawns Per Wave`))
    (set `self.Init Max Enemies Per Wave` (`self.Max Spawns Per Wave`))))

(event `Start Alarm`
  (params (AlarmReason :type Byte :default 0))
  (if (not (`self.Waves Are Initialized`))
    (set `self.Waves Are Initialized` true)
    (`KismetSystemLibrary.Delay` (`self.Time AfterAlarm`))
    (`self.Init Waves`)
    (`self.Init Start Wave Manager`)))

(event `Init Waves`
  (bind _spawn_groups (`self.Spawn Groups`))
  (bind _max_spawned_allowed (`self.Max Spawned Allowed`))
  (bind _alive_characters (`self.Alive Characters`))
  (bind _output_get (set `self.Total Enemies In Scene Before Init Wave` _alive_characters))
  (if (>= _output_get _max_spawned_allowed)
    (`self.EventTimerInitWaves`)
    (else
      (set `self.EnemiesCanSpawn` (- _max_spawned_allowed _alive_characters))
      (`self.IncreaseAndSetEnemiesPerWave`)
      (set `self.First Wave` false)
      (set `self.Wave Timer` (`KismetMathLibrary.RandomFloatInRange` (`self.Min Waves Timer`) (`self.Max Waves Timer`)))
      (`KismetArrayLibrary.Array_Clear` (`self.Spawn Groups`))
      (if (>= (`KismetArrayLibrary.Array_Length` (`self.Spawn Groups`)) 1)
        _
        (elif (== (`KismetArrayLibrary.Array_Length` (`self.Spawn Groups`)) 0)
          (`self.EventTimerInitWaves`)
          (else
            (`KismetArrayLibrary.Array_Shuffle` _spawn_groups)
            (`KismetArrayLibrary.Array_Shuffle` (`|MakeArray` (`|GetArrayItem` _spawn_groups)))
            (`self.ForEachLoopAISpawnPoints`)))))))

(event `ForEachLoopAISpawnPoints`
  (bind _outitem (`KismetArrayLibrary.Array_Random` (`/Game/Main/Blueprint/Utils/BP_SpawnGroup.Spawn Points` (`KismetArrayLibrary.Array_Random` (`self.Spawn Groups`)))))
  (set `self.Current Enemies Spawned` 0)
  (for _ (range 1 (+ (`self.EnemiesWave`) 1))
    (if (>= (`self.Current Enemies Spawned`) (`self.EnemiesCanSpawn`))
      (break)
      (elif (< (`self.Current Enemies Spawned`) (`self.EnemiesWave`))
        (`/Engine/EditorBlueprintResources/StandardMacros.IncrementInt` (`self.Current Enemies Spawned`)
          (:`  `
            (`self.Spawn New Unit` (`self.Current Waves`) (`self.Current Enemies Spawned`) _outitem)
            (`/Game/Main/Blueprint/Utils/BP_SpawnPoint.Spawn Unit` _outitem)
            (if true
              (add `/Game/Main/Blueprint/Utils/BP_SpawnPoint.AI Character Death` _outitem (`|CreateDelegate` :!event `Death AI Character`))
              (`/Engine/EditorBlueprintResources/StandardMacros.IncrementInt` (`self.Alive Characters`)))))
        (else
          (break)))))
  (if (>= (`self.Current Enemies Spawned`) (`self.EnemiesCanSpawn`))
    (`self.New Wave` (`self.Current Enemies Spawned`) (`self.Wave Timer`) (+ (`self.Total Enemies In Scene Before Init Wave`) (`self.Current Enemies Spawned`)) (`self.Current Waves`) :!label _label)
    (`/Engine/EditorBlueprintResources/StandardMacros.IncrementInt` (`self.Current Waves`)
      (:`  `
        (`self.EventTimerInitWaves`)))
    (elif (< (`self.Current Enemies Spawned`) (`self.EnemiesWave`))
      (`self.ForEachLoopAISpawnPoints`)
      (else
        (goto _label)))))

(event `Death AI Character`
  (`/Engine/EditorBlueprintResources/StandardMacros.DecrementInt` (`self.Alive Characters`)))

(event `EventTimerInitWaves`
  (bind _returnvalue (`KismetSystemLibrary.K2_SetTimerDelegate` (`|CreateDelegate` :!event `Init Waves`) (`self.Wave Timer`)))
  (set `self.Waves Timer` _returnvalue))

(event `ResetWaves`
  (bind _waves_timer (`self.Waves Timer`))
  ;[1 1 1 0.4] EventsWaveManager
  (if (`KismetSystemLibrary.K2_IsValidTimerHandle` _waves_timer)
    (`KismetSystemLibrary.K2_ClearAndInvalidateTimerHandle` _waves_timer)
    (`self.ResetVariables`)))

(event `PauseWaves`
  (params (TimerToResume :type "Float (double-precision)"))
  (bind _waves_timer (`self.Waves Timer`))
  ;[1 1 1 0.4] EventsWaveManager
  (if (`KismetSystemLibrary.K2_IsValidTimerHandle` _waves_timer)
    (`KismetSystemLibrary.K2_PauseTimerHandle` _waves_timer)
    (if (!= TimerToResume 0.0)
      (set `self.IsPaseWithTimer` true)
      (`KismetSystemLibrary.K2_SetTimerDelegate` (`|CreateDelegate` :!event `ResumeWaves`) TimerToResume)
      (else
        (set `self.IsPaseWithTimer` false)))))

(event `ResumeWaves`
  (bind _waves_timer (`self.Waves Timer`))
  ;[1 1 1 0.4] EventsWaveManager
  (if (`KismetSystemLibrary.K2_IsValidTimerHandle` _waves_timer)
    (`KismetSystemLibrary.K2_UnPauseTimerHandle` _waves_timer)
    (if (`self.IsPaseWithTimer`)
      (`self.Start Auto Resume Waves`))))

(event `ClearTimerWavesAndInitWaves`
  (params (TimerToInitWaves :type "Float (double-precision)"))
  (bind _waves_timer (`self.Waves Timer`))
  ;[1 1 1 0.4] EventsWaveManager
  (if (`KismetSystemLibrary.K2_IsValidTimerHandle` _waves_timer)
    (`KismetSystemLibrary.K2_ClearAndInvalidateTimerHandle` _waves_timer)
    (if (== TimerToInitWaves 0.0)
      (`self.Init Waves`)
      (else
        (`KismetSystemLibrary.K2_SetTimerDelegate` (`|CreateDelegate` :!event `Init Waves`) TimerToInitWaves)))))

(event `SetWaveSpawnTimer`
  (params (MinWaveSpawnTimer :type "Float (double-precision)") (MaxWaveSpawnTimer :type "Float (double-precision)"))
  ;[1 1 1 0.4] EventsWaveManager
  (set `self.Min Waves Timer` MinWaveSpawnTimer)
  (set `self.Max Waves Timer` MaxWaveSpawnTimer))

(event `SetIncrementPerWave`
  (params (IncrementPerWave :type Integer))
  ;[1 1 1 0.4] EventsWaveManager
  (set `self.Increment Per Wave` IncrementPerWave))

(fn `IncreaseAndSetEnemiesPerWave`
  (if (== (`self.Increment Per Wave`) 0)
    _
    (elif (`self.First Wave`)
      _
      (elif (or (< (`self.Current Time Increment`) (`self.Times Increased`)) (== (`self.Times Increased`) 0))
        (set `self.Min Spawns Per Wave` (+ (`self.Min Spawns Per Wave`) (`self.Increment Per Wave`)))
        (set `self.Max Spawns Per Wave` (+ (`self.Max Spawns Per Wave`) (`self.Increment Per Wave`)))
        (`/Engine/EditorBlueprintResources/StandardMacros.IncrementInt` (`self.Current Time Increment`)
          (:`  `
            _)))))
  (set `self.EnemiesWave` (`KismetMathLibrary.RandomIntegerInRange` (`self.Min Spawns Per Wave`) (`self.Max Spawns Per Wave`))))

(fn `ResetVariables`
  (set `self.Min Spawns Per Wave` (`self.Init Min Enemies Per Wave`))
  (set `self.Max Spawns Per Wave` (`self.Init Max Enemies Per Wave`))
  (set `self.Current Time Increment` 0)
  (set `self.Current Waves` 0))

(fn `UserConstructionScript`
  (if (> (`self.Min Spawns Per Wave`) (`self.Max Spawns Per Wave`))
    (set `self.Min Spawns Per Wave` (`self.Max Spawns Per Wave`)))
  (if (> (`self.Min Waves Timer`) (`self.Max Waves Timer`))
    (set `self.Min Waves Timer` (`self.Max Waves Timer`))))