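; BP_TrafficSpline is a traffic spawner that feeds random vehicles onto its spline.
; When AutoActivate is set, BeginPlay starts a looping fixed-interval timer that calls ActivateTraffic, which also prints a debug string.
; Each call spawns a random TrafficVehicles class at the first spline point's local-space transform, passing it the spline and Duration.
; The randomized interval from MinTimeBetweenVehicles and MaxTimeBetweenVehicles is left unconnected.
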(event `self.ReceiveBeginPlay`
  (if (`self.Auto Activate`)
    (`KismetSystemLibrary.K2_SetTimerDelegate` (delegate `Activate Traffic`) 5.0 true)))

(event `Activate Traffic`
  (bind _spline (`self.Spline`))
  (`KismetSystemLibrary.PrintString` "ENTRADA" true true (struct :`R` 0.94 :`G` 0.586711 :`A` 1.0))
  (`|SpawnActorFromClass` (`KismetArrayLibrary.Array_Random` (`.TrafficVehicles_8_50CD49734AE72DFFDC891EAE3F70C4CF` (break `/Game/Main/Blueprint/Vehicles/TrafficSystem/ST_TrafficVehicles` (`self.Traffic Vehicles`)))) (`SplineComponent.GetTransformAtSplinePoint` _spline 0 "Local" false) "Undefined" "OverrideRootScale" null _spline (`self.Duration`) null))

(fn `UserConstructionScript`)