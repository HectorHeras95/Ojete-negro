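; BP_TrafficVehicle is a traffic vehicle actor that drives itself along a spline once and destroys itself at the end.
; On BeginPlay it plays the Movement timeline, with the play rate set to the inverse of Duration to control travel time.
; Separate Location and Rotation tracks map to distances along the spline, setting the world transform each update with sweep enabled.
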(event `self.ReceiveBeginPlay`
  (`self.ActivateMovement`))

(event `ActivateMovement`
  (bind _spline (`self.Spline`))
  (bind _returnvalue (`SplineComponent.GetSplineLength` _spline))
  (`TimelineComponent.SetPlayRate` (`self.Movement`) (/ 1.0 (`self.Duration`)))
  (bind (_direction _location _rotation) (`Timeline|Movement` :!via `PlayFromStart`)
    (:`Update`
      (`self.K2_SetActorLocationAndRotation` self (`SplineComponent.GetLocationAtDistanceAlongSpline` _spline (`KismetMathLibrary.Lerp` 0.0 _returnvalue _location) "World") (`SplineComponent.GetRotationAtDistanceAlongSpline` _spline (`KismetMathLibrary.Lerp` 0.0 _returnvalue _rotation) "World") true false))
    (:`Finished`
      (`self.K2_DestroyActor`))))

(fn `UserConstructionScript`)